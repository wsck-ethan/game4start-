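; BP_launcher is an actor that spawns a BP_ball whenever the 1 key is pressed.
; It prints a "press 1" prompt at BeginPlay, then spawns each ball at its Cube component's world location, using only the position.
; No launch force or velocity is applied here, and the overlap, Tick and construction logic hold no custom behavior.
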(event `self.ReceiveBeginPlay`
  (`KismetSystemLibrary.PrintString` "press 1"))

(event `Key|One`
  (params (Key :type "Key Structure"))
  (:`Pressed`
    (`|SpawnActorFromClass` "/Game/ethan/blueprints_clas/BP_ball.BP_ball_C" (`KismetMathLibrary.Conv_VectorToTransform` (`SceneComponent.K2_GetComponentLocation` (`self.Cube`))) "Undefined" "MultiplyWithRoot" null null)))

(fn `UserConstructionScript`
  (`parent.UserConstructionScript`))