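; BP_launcher is an actor that spawns a BP_ball at the third-person character's location when the primary action is pressed.
; On BeginPlay it prints a "press 1" prompt and turns off collision on Cube1 and Cube2.
; It applies no launch velocity to the spawned ball.
; Nodes for Cube3 and Cube4 collision and for disabling physics on all four cubes are unconnected and never run.
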(event `self.ReceiveBeginPlay`
  (`KismetSystemLibrary.PrintString` "press 1")
  (`PrimitiveComponent.SetCollisionEnabled` (`self.Cube1`) "NoCollision")
  (`PrimitiveComponent.SetCollisionEnabled` (`self.Cube2`) "NoCollision"))

(event `self.primaryAction`
  (params (`held down` :type Boolean))
  (if `held down`
    (bind _returnvalue (`GameplayStatics.GetActorOfClass` "/Game/ThirdPerson/Blueprints/BP_ThirdPersonCharacter.BP_ThirdPersonCharacter_C"))
    (`|SpawnActorFromClass` "/Game/ethan/blueprints_clas/BP_ball.BP_ball_C" (`KismetMathLibrary.Conv_VectorToTransform` (`self.K2_GetActorLocation` _returnvalue)) "Undefined" "MultiplyWithRoot" null null)))

(fn `UserConstructionScript`
  (`parent.UserConstructionScript`))