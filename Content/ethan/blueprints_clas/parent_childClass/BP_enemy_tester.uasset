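; BP_enemy_tester is a test Blueprint that repeatedly damages every BP_enemy in the level.
; On BeginPlay it gathers all BP_enemy actors, prints their count, then calls TakeDamage on each with a small random amount and prints its array index.
; After a two-second Delay it calls its GiveDamage custom event, which re-enters the search, so the cycle repeats indefinitely.
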(event `self.ReceiveBeginPlay`
  (bind _outactors (`GameplayStatics.GetAllActorsOfClass` "/Game/ethan/blueprints_clas/parent_childClass/BP_enemy.BP_enemy_C" :!label _label)) ; find all enemies
  (`KismetSystemLibrary.PrintString` (`KismetStringLibrary.Concat_StrStr` "there are " (`KismetStringLibrary.Conv_IntToString` (`KismetArrayLibrary.Array_Length` _outactors)) "enemies in the level") true true (struct :`G` 0.66 :`B` 1.0 :`A` 1.0) 5.0)
  (for (_array_element _array_index) _outactors
    (`/Game/ethan/blueprints_clas/parent_childClass/BP_enemy.take damage` _array_element (`KismetMathLibrary.RandomFloatInRange` 0.1 0.5))
    (`KismetSystemLibrary.PrintString` (`KismetStringLibrary.Concat_StrStr` "array index=" (`KismetStringLibrary.Conv_IntToString` _array_index)) true true (struct :`G` 0.66 :`B` 1.0 :`A` 1.0) 50.0))
  (`KismetSystemLibrary.PrintString` "we have given damage to all enemies")
  (`KismetSystemLibrary.Delay` 2.0)
  (`self.give damage`))

(event `give damage`
  (goto _label))

(fn `UserConstructionScript`)