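; BP_exsplosion is a short-lived explosion actor that applies a physics push when spawned.
; On BeginPlay its RadialForce component fires a single impulse, and a lifespan timer removes the actor a few seconds later.
; The OnPrime and component-activation events are empty.
; Unwired leftover chains hold a delayed force activation and an older detonation sequence with particles, sound, mesh hiding and destruction.
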(event `OnPrime`)

(event `self.RadialForce.OnComponentActivated`
  (params (Component :type "ActorComponent Object Reference") (bReset :type Boolean)))

(event `self.ReceiveBeginPlay`
  (`RadialForceComponent.FireImpulse` (`self.RadialForce`))
  (`self.SetLifeSpan` 4.0))

(fn `UserConstructionScript`)