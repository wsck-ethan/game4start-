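; Grenade actor that explodes on a five-second fuse started by its OnPrime event.
; When the fuse ends it activates its RadialForce component, whose activation event handles the detonation.
; That event spawns an emitter and plays a sound at the mesh, fires the radial impulse, hides the mesh, then destroys the actor after a short delay.
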(event `OnPrime`
  (`KismetSystemLibrary.Delay` 5.0)
  (`ActorComponent.Activate` (`self.RadialForce`) false))

(event `self.RadialForce.OnComponentActivated`
  (params (Component :type "ActorComponent Object Reference") (bReset :type Boolean))
  (bind _meshcomp (`self.meshcomp`))
  (bind _returnvalue (`SceneComponent.K2_GetComponentLocation` _meshcomp))
  (`GameplayStatics.SpawnEmitterAtLocation` null _returnvalue (`SceneComponent.K2_GetComponentRotation` _meshcomp))
  (`GameplayStatics.PlaySoundAtLocation` null _returnvalue (struct) 1.0 1.0 0.0 null null null null)
  (`RadialForceComponent.FireImpulse` (`self.RadialForce`))
  (`SceneComponent.SetHiddenInGame` (`self.meshcomp`) true false)
  (`KismetSystemLibrary.Delay` 0.4)
  (`self.K2_DestroyActor`))

(fn `UserConstructionScript`)