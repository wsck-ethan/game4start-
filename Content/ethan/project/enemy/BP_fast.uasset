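; BP_fast is a fast enemy variant that extends a parent Blueprint and bursts into high speed when it spots the player.
; On BeginPlay it runs the parent logic, then randomizes its capsule's world scale for size variety.
; When PawnSensing sees BP_ThirdPersonCharacter, it drops MaxSpeed briefly as a short wind-up, then raises it sharply, with no reset afterward in this graph.
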(event `self.ReceiveBeginPlay`
  (bind _capsulecomponent (`self.CapsuleComponent`))
  (`parent.ReceiveBeginPlay`)
  (`SceneComponent.SetWorldScale3D` _capsulecomponent (`KismetMathLibrary.Conv_DoubleToVector` (- (`CapsuleComponent.GetShapeScale` _capsulecomponent) (`KismetMathLibrary.RandomFloatInRange` -0.5 0.5)))))

(event `self.PawnSensing.OnSeePawn`
  (params (Pawn :type "Pawn Object Reference"))
  (cast `/Game/ThirdPerson/Blueprints/BP_ThirdPersonCharacter` Pawn)
  (set `self.max speed` 100.0)
  (`KismetSystemLibrary.Delay` 0.2)
  (set `self.max speed` 1100.0))

(fn `UserConstructionScript`
  (`parent.UserConstructionScript`))