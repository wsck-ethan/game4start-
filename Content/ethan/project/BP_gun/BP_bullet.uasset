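; BP_bullet is a projectile actor for a gun, moved by a ProjectileMovement component.
; On BeginPlay it copies the component's speed, bounce, friction and homing settings into its own variables, which nothing else in these graphs reads.
; It then destroys itself after a short fixed delay, with no hit or damage logic in the graphs.
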(event `self.ReceiveBeginPlay`
  (bind _projectilemovement (`self.ProjectileMovement`))
  (set `self.projectile initial speed` (`ProjectileMovementComponent.InitialSpeed` _projectilemovement))
  (set `self.projectile max speed` (`MovementComponent.GetMaxSpeed` _projectilemovement))
  (set `self.bounce` (`ProjectileMovementComponent.Bounciness` _projectilemovement))
  (set `self.friction` (`ProjectileMovementComponent.Friction` _projectilemovement))
  (set `self.homing` (`ProjectileMovementComponent.bIsHomingProjectile` _projectilemovement))
  (`KismetSystemLibrary.Delay` 1.0)
  (`self.K2_DestroyActor`))

(fn `UserConstructionScript`)