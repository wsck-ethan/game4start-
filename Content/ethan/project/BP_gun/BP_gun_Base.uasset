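; BP_gun_Base is a gun actor that can be picked up and dropped.
; Pickup disables the Cube's collision and physics, then attaches to the passed mesh's "shoulder gun" socket; drop detaches it, restores both and adds a force.
; Its primary action only copies projectile and damage settings from a BP_bullet found in the world, without spawning or firing anything.
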(event `pickup`
  (params (mesh :type "SceneComponent Object Reference"))
  (`KismetSystemLibrary.PrintString` "Picked Up" true true (struct :`G` 1.0 :`B` 0.253051 :`A` 1.0))
  (`PrimitiveComponent.SetCollisionEnabled` (`self.Cube`) "NoCollision") ; dont push us off map
  (`PrimitiveComponent.SetSimulatePhysics` (`self.Cube`) false)
  (`self.K2_AttachToComponent` mesh "shoulder gun" "SnapToTarget" "SnapToTarget" "KeepRelative")
  (`self.K2_SetActorRotation` (struct :`Pitch` -10.0 :`Yaw` -90.0 :`Roll` -10.0)))

(event `drop`
  (`KismetSystemLibrary.PrintString` "Dropped" true true (struct :`R` 0.122709 :`G` 1.0 :`B` 0.306853 :`A` 1.0))
  (`SceneComponent.K2_DetachFromComponent` (`self.Cube`) "KeepWorld" "KeepWorld" "KeepRelative" true)
  (`PrimitiveComponent.SetCollisionEnabled` (`self.Cube`) "QueryAndPhysics")
  (`PrimitiveComponent.SetSimulatePhysics` (`self.Cube`) true)
  (`PrimitiveComponent.AddForce` (`self.Cube`) (1000.0 500.0 0.0) "None" false))

(event `primaryAction`
  (params (`held down` :type Boolean))
  (bind _returnvalue (`GameplayStatics.GetActorOfClass` "/Game/ethan/project/BP_gun/BP_bullet.BP_bullet_C"))
  (set `self.gun bullet projectile speed` (`/Game/ethan/project/BP_gun/BP_bullet.projectile initial speed` _returnvalue))
  (set `self.gun bullet max speed` (`/Game/ethan/project/BP_gun/BP_bullet.projectile max speed` _returnvalue))
  (set `self.projectile Bounce` (`/Game/ethan/project/BP_gun/BP_bullet.bounce` _returnvalue))
  (set `self.projectile friction` (`/Game/ethan/project/BP_gun/BP_bullet.friction` _returnvalue))
  (set `self.projectile is homing` (`/Game/ethan/project/BP_gun/BP_bullet.homing` _returnvalue))
  (set `self.damage bullet` (`/Game/ethan/project/BP_gun/BP_bullet.damage` _returnvalue)))

(fn `UserConstructionScript`)