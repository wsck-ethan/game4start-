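; Gun Blueprint that aims with the player camera and damages enemies when its primary action fires.
; PrimaryAction rotates the Cube component to match the third-person character's FollowCamera and plays a 2D sound.
; It then loops over all BP_base_enemy actors and subtracts Damage from the Health of the one matching the character's HitActorLineTrace.
; The gun runs no trace itself, relying on the character's stored hit actor.
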(event `self.primaryAction`
  (params (`held down` :type Boolean))
  (bind _asbp_third_person_character (cast `/Game/ThirdPerson/Blueprints/BP_ThirdPersonCharacter` (`GameplayStatics.GetPlayerCharacter` 0)))
  (`SceneComponent.K2_SetWorldRotation` (`self.Cube`) (`SceneComponent.K2_GetComponentRotation` (`/Game/ThirdPerson/Blueprints/BP_ThirdPersonCharacter.FollowCamera` _asbp_third_person_character)) false false)
  (`GameplayStatics.PlaySound2D` null 1.0 1.0 0.0 null null)
  (bind _outactors (`GameplayStatics.GetAllActorsOfClass` "/Game/ethan/project/enemy/BP_base_enemy.BP_base_enemy_C"))
  (for _array_element _outactors
    (if (== (`/Game/ThirdPerson/Blueprints/BP_ThirdPersonCharacter.Hit Actor Line trace` _asbp_third_person_character) _array_element)
      (set `/Game/ethan/project/enemy/BP_base_enemy.health` (- (`/Game/ethan/project/enemy/BP_base_enemy.health` _array_element) (`self.damage`)) _array_element))))

(fn `UserConstructionScript`
  (`parent.UserConstructionScript`))