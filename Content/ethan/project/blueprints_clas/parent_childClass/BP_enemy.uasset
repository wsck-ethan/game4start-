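; BP_enemy is a basic enemy actor with a health value that takes damage and destroys itself on death.
; It prints a greeting on BeginPlay, and its takedamage event prints a reaction and subtracts the passed amount from Health.
; The CheckIfDead function then reports whether Health is at or below zero, and a true result destroys the actor.
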(event `self.ReceiveBeginPlay`
  (`KismetSystemLibrary.PrintString` "Hello, time to die"))

(event `take damage`
  (params (`buy amount` :type "Float (double-precision)" :default 0.2))
  (`KismetSystemLibrary.PrintString` "ouch")
  (bind _output_get (set `self.health` (- (`self.health`) `buy amount`)))
  (if (`self.checkIfDead` _output_get)
    (`self.K2_DestroyActor`)))

(fn `checkIfDead`
  (params (health :type "Float (double-precision)"))
  (returns (`is dead` :type Boolean))
  (return (<= health 0.0)))

(fn `UserConstructionScript`)