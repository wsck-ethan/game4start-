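; BP_shootsBall is an item that fires physics balls on its primary action, with a limited shot count.
; Each use launches the third-person character upward and spawns a BP_ball at that character's JumpingItem transform with a fixed world-space velocity.
; A Balls counter increments and prints per shot; once it passes the limit, the next use sets a short lifespan to remove the item.
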(event `self.ReceiveBeginPlay`)

(event `self.primaryAction`
  (params (`held down` :type Boolean))
  (if (<= (`self.balls`) 10)
    (bind _returnvalue (`GameplayStatics.GetActorOfClass` "/Game/ThirdPerson/Blueprints/BP_ThirdPersonCharacter.BP_ThirdPersonCharacter_C"))
    (`Character.LaunchCharacter` _returnvalue (0.0 0.0 200.0) false false)
    (bind _returnvalue_2 (`|SpawnActorFromClass` "/Game/ethan/project/blueprints_clas/BP_ball.BP_ball_C" (`SceneComponent.K2_GetComponentToWorld` (`/Game/ThirdPerson/Blueprints/BP_ThirdPersonCharacter.jumping_item` _returnvalue)) "Undefined" "MultiplyWithRoot" null null))
    (`PrimitiveComponent.SetPhysicsLinearVelocity` (`/Game/ethan/project/blueprints_clas/BP_ball.Sphere` _returnvalue_2) (0.0 100.0 0.0) false "None")
    (bind _output_get (set `self.balls` (+ 1 (`self.balls`))))
    (`KismetSystemLibrary.PrintString` (`KismetStringLibrary.Conv_Int64ToString` _output_get))
    (else
      (`self.SetLifeSpan` 1.0))))

(fn `UserConstructionScript`
  (`parent.UserConstructionScript`))