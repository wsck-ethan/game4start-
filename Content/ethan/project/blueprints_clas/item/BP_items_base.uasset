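; Base item Blueprint for objects a character can pick up, hold and drop.
; Pickup disables collision and physics on its Cube, then attaches the given mesh's item_socket_r socket as the Cube's parent.
; Drop detaches the Cube, restores collision and physics, and applies a fixed force.
; primaryAction takes a held-down input but is empty here, as are BeginPlay and the construction script.
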(event `self.ReceiveBeginPlay`)

(event `pickup`
  (params (mesh :type "SceneComponent Object Reference"))
  (`KismetSystemLibrary.PrintString` "Picked Up" true true (struct :`G` 1.0 :`B` 0.253051 :`A` 1.0))
  (`PrimitiveComponent.SetCollisionEnabled` (`self.Cube`) "NoCollision") ; dont push us off map
  (`PrimitiveComponent.SetSimulatePhysics` (`self.Cube`) false)
  (`self.K2_AttachToComponent` mesh "item_socket_r" "SnapToTarget" "SnapToTarget" "KeepRelative"))

(event `drop`
  (`KismetSystemLibrary.PrintString` "Dropped" true true (struct :`R` 0.122709 :`G` 1.0 :`B` 0.306853 :`A` 1.0))
  (`SceneComponent.K2_DetachFromComponent` (`self.Cube`) "KeepWorld" "KeepWorld" "KeepRelative" true)
  (`PrimitiveComponent.SetCollisionEnabled` (`self.Cube`) "QueryAndPhysics")
  (`PrimitiveComponent.SetSimulatePhysics` (`self.Cube`) true)
  (`PrimitiveComponent.AddForce` (`self.Cube`) (1000.0 500.0 0.0) "None" false))

(event `primaryAction`
  (params (`held down` :type Boolean)))

(fn `UserConstructionScript`)