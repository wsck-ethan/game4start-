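; BP_potion is a single-use health potion item that heals the player character.
; On PrimaryAction it adds HealthAdded to the Health of player 0's BP_ThirdPersonCharacter, sets a Used flag, then caps Health at MaxHealth.
; Once used, further actions only print "drank".
; The construction script only calls its parent, and the overlap event is disabled.
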(event `self.primaryAction`
  (params (`held down` :type Boolean))
  (if (`self.used`)
    (`KismetSystemLibrary.PrintString` "drank")
    (else
      (bind _asbp_third_person_character (cast `/Game/ThirdPerson/Blueprints/BP_ThirdPersonCharacter` (`GameplayStatics.GetPlayerCharacter` 0)))
      (set `/Game/ThirdPerson/Blueprints/BP_ThirdPersonCharacter.health` (+ (`self.health added`) (`/Game/ThirdPerson/Blueprints/BP_ThirdPersonCharacter.health` _asbp_third_person_character)) _asbp_third_person_character)
      (set `self.used` true)
      (if (> (`/Game/ThirdPerson/Blueprints/BP_ThirdPersonCharacter.health` _asbp_third_person_character) (`/Game/ThirdPerson/Blueprints/BP_ThirdPersonCharacter.max health` _asbp_third_person_character))
        (set `/Game/ThirdPerson/Blueprints/BP_ThirdPersonCharacter.health` (`/Game/ThirdPerson/Blueprints/BP_ThirdPersonCharacter.max health` _asbp_third_person_character) _asbp_third_person_character)))))

(fn `UserConstructionScript`
  (`parent.UserConstructionScript`))